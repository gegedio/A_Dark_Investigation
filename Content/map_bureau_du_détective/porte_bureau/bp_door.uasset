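; Interactive office door that the first-person player can open and close with an input action.
; A box trigger enables the door's input while the character is inside and disables it on exit.
; The input plays or reverses a timeline that offsets the door's yaw from the rotation saved at BeginPlay.
; The timeline's track value also updates the closed flag that selects the direction of the next press.
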(event `self.ReceiveBeginPlay`
  ;[1 0 0.09139] info rotation et location de la porte au début du jeux
  (set `self.rotation départ` (`SceneComponent.RelativeRotation` (`self.porte_nv`))))

(event `self.Box.OnComponentBeginOverlap`
  (params (OverlappedComponent :type "PrimitiveComponent Object Reference") (OtherActor :type "Actor Object Reference") (OtherComp :type "PrimitiveComponent Object Reference") (OtherBodyIndex :type Integer) (bFromSweep :type Boolean) (SweepResult :type "HitResult Structure (by ref)"))
  ;[0.3456 0.3105 1] reconaitre le personage dans la boxe
  (cast `/Game/FirstPersonBP/Blueprints/FirstPersonCharacter` OtherActor)
  (`self.EnableInput` (`GameplayStatics.GetPlayerController` 0)))

(event `InputAction|overture porte`
  (params (Key :type "Key Structure"))
  (:`Pressed`
    (if (`self.porte fermé`)
      (bind (_direction _newtrack_0) (`Timeline|timeline 0` :!label _label)
        (:`Update`
          (`SceneComponent.K2_SetRelativeRotation` (`self.porte_nv`) (`KismetMathLibrary.MakeRotator` (.roll (`self.rotation départ`)) (.pitch (`self.rotation départ`)) (+ _newtrack_0 (.yaw (`self.rotation départ`)))) false false)
          (set `self.porte fermé` (< _newtrack_0 1.0))))
      (else
        (goto _label :!via `Reverse`)))))

(event `self.Box.OnComponentEndOverlap`
  (params (OverlappedComponent :type "PrimitiveComponent Object Reference") (OtherActor :type "Actor Object Reference") (OtherComp :type "PrimitiveComponent Object Reference") (OtherBodyIndex :type Integer))
  ;[0.3456 0.3105 1] reconaitre le personage dans la boxe
  (cast `/Game/FirstPersonBP/Blueprints/FirstPersonCharacter` OtherActor)
  (`self.DisableInput` (`GameplayStatics.GetPlayerController` 0)))

(fn `UserConstructionScript`)